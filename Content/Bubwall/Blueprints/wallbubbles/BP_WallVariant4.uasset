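; Bubble wall variant that spawns a fixed, hand-authored pattern of colored bubble actors when play begins.
; On BeginPlay, a single Sequence spawns one green, yellow, red, blue or purple bubble at the world location of each of its 25 numbered Box components.
; The color layout is hardcoded per box, with no randomization, loop or further logic after spawning.
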(event EventBeginPlay
  (Utilities|FlowControl|Sequence
    (:then_0
      (Game|SpawnActorfromClass "/Game/Bubwall/Blueprints/wallbubbles/greenbubble.greenbubble_C" (Math|Transform|MakeTransform (Transformation|GetWorldLocation (Variables|Default|GetBox1)) "0, 0, 0" "1.000000,1.000000,1.000000") "Undefined" "MultiplyWithRoot" 0 0))
    (:then_1
      (Game|SpawnActorfromClass "/Game/Bubwall/Blueprints/wallbubbles/greenbubble.greenbubble_C" (Math|Transform|MakeTransform (Transformation|GetWorldLocation (Variables|Default|GetBox2)) "0, 0, 0" "1.000000,1.000000,1.000000") "Undefined" "MultiplyWithRoot" 0 0))
    (:then_2
      (Game|SpawnActorfromClass "/Game/Bubwall/Blueprints/wallbubbles/greenbubble.greenbubble_C" (Math|Transform|MakeTransform (Transformation|GetWorldLocation (Variables|Default|GetBox6)) "0, 0, 0" "1.000000,1.000000,1.000000") "Undefined" "MultiplyWithRoot" 0 0))
    (:then_3
      (Game|SpawnActorfromClass "/Game/Bubwall/Blueprints/wallbubbles/greenbubble.greenbubble_C" (Math|Transform|MakeTransform (Transformation|GetWorldLocation (Variables|Default|GetBox11)) "0, 0, 0" "1.000000,1.000000,1.000000") "Undefined" "MultiplyWithRoot" 0 0))
    (:then_4
      (Game|SpawnActorfromClass "/Game/Bubwall/Blueprints/wallbubbles/greenbubble.greenbubble_C" (Math|Transform|MakeTransform (Transformation|GetWorldLocation (Variables|Default|GetBox16)) "0, 0, 0" "1.000000,1.000000,1.000000") "Undefined" "MultiplyWithRoot" 0 0))
    (:then_5
      (Game|SpawnActorfromClass "/Game/Bubwall/Blueprints/wallbubbles/greenbubble.greenbubble_C" (Math|Transform|MakeTransform (Transformation|GetWorldLocation (Variables|Default|GetBox21)) "0, 0, 0" "1.000000,1.000000,1.000000") "Undefined" "MultiplyWithRoot" 0 0))
    (:then_6
      (Game|SpawnActorfromClass "/Game/Bubwall/Blueprints/wallbubbles/greenbubble.greenbubble_C" (Math|Transform|MakeTransform (Transformation|GetWorldLocation (Variables|Default|GetBox22)) "0, 0, 0" "1.000000,1.000000,1.000000") "Undefined" "MultiplyWithRoot" 0 0))
    (:then_7
      (Game|SpawnActorfromClass "/Game/Bubwall/Blueprints/wallbubbles/yellowbubble.yellowbubble_C" (Math|Transform|MakeTransform (Transformation|GetWorldLocation (Variables|Default|GetBox3)) "0, 0, 0" "1.000000,1.000000,1.000000") "Undefined" "MultiplyWithRoot" 0 0))
    (:then_8
      (Game|SpawnActorfromClass "/Game/Bubwall/Blueprints/wallbubbles/yellowbubble.yellowbubble_C" (Math|Transform|MakeTransform (Transformation|GetWorldLocation (Variables|Default|GetBox12)) "0, 0, 0" "1.000000,1.000000,1.000000") "Undefined" "MultiplyWithRoot" 0 0))
    (:then_9
      (Game|SpawnActorfromClass "/Game/Bubwall/Blueprints/wallbubbles/redbubble.redbubble_C" (Math|Transform|MakeTransform (Transformation|GetWorldLocation (Variables|Default|GetBox14)) "0, 0, 0" "1.000000,1.000000,1.000000") "Undefined" "MultiplyWithRoot" 0 0))
    (:then_10
      (Game|SpawnActorfromClass "/Game/Bubwall/Blueprints/wallbubbles/redbubble.redbubble_C" (Math|Transform|MakeTransform (Transformation|GetWorldLocation (Variables|Default|GetBox23)) "0, 0, 0" "1.000000,1.000000,1.000000") "Undefined" "MultiplyWithRoot" 0 0))
    (:then_11
      (Game|SpawnActorfromClass "/Game/Bubwall/Blueprints/wallbubbles/bluebubble.bluebubble_C" (Math|Transform|MakeTransform (Transformation|GetWorldLocation (Variables|Default|GetBox4)) "0, 0, 0" "1.000000,1.000000,1.000000") "Undefined" "MultiplyWithRoot" 0 0))
    (:then_12
      (Game|SpawnActorfromClass "/Game/Bubwall/Blueprints/wallbubbles/bluebubble.bluebubble_C" (Math|Transform|MakeTransform (Transformation|GetWorldLocation (Variables|Default|GetBox5)) "0, 0, 0" "1.000000,1.000000,1.000000") "Undefined" "MultiplyWithRoot" 0 0))
    (:then_13
      (Game|SpawnActorfromClass "/Game/Bubwall/Blueprints/wallbubbles/bluebubble.bluebubble_C" (Math|Transform|MakeTransform (Transformation|GetWorldLocation (Variables|Default|GetBox10)) "0, 0, 0" "1.000000,1.000000,1.000000") "Undefined" "MultiplyWithRoot" 0 0))
    (:then_14
      (Game|SpawnActorfromClass "/Game/Bubwall/Blueprints/wallbubbles/bluebubble.bluebubble_C" (Math|Transform|MakeTransform (Transformation|GetWorldLocation (Variables|Default|GetBox15)) "0, 0, 0" "1.000000,1.000000,1.000000") "Undefined" "MultiplyWithRoot" 0 0))
    (:then_15
      (Game|SpawnActorfromClass "/Game/Bubwall/Blueprints/wallbubbles/bluebubble.bluebubble_C" (Math|Transform|MakeTransform (Transformation|GetWorldLocation (Variables|Default|GetBox20)) "0, 0, 0" "1.000000,1.000000,1.000000") "Undefined" "MultiplyWithRoot" 0 0))
    (:then_16
      (Game|SpawnActorfromClass "/Game/Bubwall/Blueprints/wallbubbles/bluebubble.bluebubble_C" (Math|Transform|MakeTransform (Transformation|GetWorldLocation (Variables|Default|GetBox24)) "0, 0, 0" "1.000000,1.000000,1.000000") "Undefined" "MultiplyWithRoot" 0 0))
    (:then_17
      (Game|SpawnActorfromClass "/Game/Bubwall/Blueprints/wallbubbles/bluebubble.bluebubble_C" (Math|Transform|MakeTransform (Transformation|GetWorldLocation (Variables|Default|GetBox25)) "0, 0, 0" "1.000000,1.000000,1.000000") "Undefined" "MultiplyWithRoot" 0 0))
    (:then_18
      (Game|SpawnActorfromClass "/Game/Bubwall/Blueprints/wallbubbles/purplebubble.purplebubble_C" (Math|Transform|MakeTransform (Transformation|GetWorldLocation (Variables|Default|GetBox7)) "0, 0, 0" "1.000000,1.000000,1.000000") "Undefined" "MultiplyWithRoot" 0 0))
    (:then_19
      (Game|SpawnActorfromClass "/Game/Bubwall/Blueprints/wallbubbles/purplebubble.purplebubble_C" (Math|Transform|MakeTransform (Transformation|GetWorldLocation (Variables|Default|GetBox8)) "0, 0, 0" "1.000000,1.000000,1.000000") "Undefined" "MultiplyWithRoot" 0 0))
    (:then_20
      (Game|SpawnActorfromClass "/Game/Bubwall/Blueprints/wallbubbles/purplebubble.purplebubble_C" (Math|Transform|MakeTransform (Transformation|GetWorldLocation (Variables|Default|GetBox9)) "0, 0, 0" "1.000000,1.000000,1.000000") "Undefined" "MultiplyWithRoot" 0 0))
    (:then_21
      (Game|SpawnActorfromClass "/Game/Bubwall/Blueprints/wallbubbles/purplebubble.purplebubble_C" (Math|Transform|MakeTransform (Transformation|GetWorldLocation (Variables|Default|GetBox13)) "0, 0, 0" "1.000000,1.000000,1.000000") "Undefined" "MultiplyWithRoot" 0 0))
    (:then_22
      (Game|SpawnActorfromClass "/Game/Bubwall/Blueprints/wallbubbles/purplebubble.purplebubble_C" (Math|Transform|MakeTransform (Transformation|GetWorldLocation (Variables|Default|GetBox17)) "0, 0, 0" "1.000000,1.000000,1.000000") "Undefined" "MultiplyWithRoot" 0 0))
    (:then_23
      (Game|SpawnActorfromClass "/Game/Bubwall/Blueprints/wallbubbles/purplebubble.purplebubble_C" (Math|Transform|MakeTransform (Transformation|GetWorldLocation (Variables|Default|GetBox18)) "0, 0, 0" "1.000000,1.000000,1.000000") "Undefined" "MultiplyWithRoot" 0 0))
    (:then_24
      (Game|SpawnActorfromClass "/Game/Bubwall/Blueprints/wallbubbles/purplebubble.purplebubble_C" (Math|Transform|MakeTransform (Transformation|GetWorldLocation (Variables|Default|GetBox19)) "0, 0, 0" "1.000000,1.000000,1.000000") "Undefined" "MultiplyWithRoot" 0 0))))

(fn ConstructionScript)